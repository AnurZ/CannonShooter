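; Player controller that lets the player aim and fire a possessed BP_Cannon.
; The RaiseCannon axis pitches the cannon's Arrow component by adding relative rotation scaled from the input, with no clamping or frame-time scaling.
; The Fire action spawns a BP_Projectile at the Barrel's world transform and launches it with a physics impulse along the barrel's forward direction.
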(event EventBeginPlay)

(event EventTick
  (params (DeltaSeconds :type Float%20%28single-precision%29)))

(event Input|ActionEvents|InputActionFire
  (params (Key :type Key%20Structure))
  (:Pressed
    (bind _asbp_cannon (Utilities|Casting|CastToBP_Cannon (Pawn|GetControlledPawn)))
    (bind _returnvalue (Game|SpawnActorfromClass "/Game/BP_Projectile.BP_Projectile_C" (Math|Transform|MakeTransform (.location (Transformation|GetWorldTransform (Variables|/Game/BP_Cannon.BP_Cannon_C|GetBarrel _asbp_cannon))) (.rotation (Transformation|GetWorldTransform (Variables|/Game/BP_Cannon.BP_Cannon_C|GetBarrel _asbp_cannon))) "1,1,1") "Undefined" 0 0))
    (Physics|AddImpulse (Variables|/Game/BP_Projectile.BP_Projectile_C|GetSphere _returnvalue) (Math|Vector|RotateVector (Math|Vector|MakeVector 5e+03 0.0 0.0) (Transformation|GetWorldRotation (Variables|/Game/BP_Cannon.BP_Cannon_C|GetBarrel _asbp_cannon))) "None" false)))

(event Input|AxisEvents|InputAxisRaiseCannon
  (params (AxisValue :type Float%20%28single-precision%29))
  (if (!= AxisValue 0.0)
    (bind _asbp_cannon (Utilities|Casting|CastToBP_Cannon (Pawn|GetControlledPawn)))
    (Transformation|AddRelativeRotation (Variables|/Game/BP_Cannon.BP_Cannon_C|GetArrow _asbp_cannon) (Math|Rotator|MakeRotator 0.0 (* AxisValue 2.0) 0.0) false false)))

(fn ConstructionScript)